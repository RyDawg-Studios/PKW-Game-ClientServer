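; Base dialogue tree that holds a list of dialogue entries, with empty Init and OnDialogueComplete events.
; AddLine appends an entry and returns its index, AddOption attaches replies to an existing entry, and ClearDialogue empties the list.
; Helpers increment a capped times-spoken counter and pick random integers, avoiding immediate repeats by removing the last pick from a refreshed pool.
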(event Custom|Init)

(event Custom|On%20Dialogue%20Complete)

(fn AddLine
  (params (Dialogue :type Array%20of%20Texts) (Next? :type E_DialogueNext%20Enum :default "NewEnumerator0"))
  (bind _returnvalue (Utilities|Array|Add (Variables|Default|GetDialogue%20Content) (Utilities|Struct|MakeS_DialogueContent Dialogue Next?)))
  (return _returnvalue))

(fn AddOption
  (params (Index :type Integer) (Replies :type Array%20of%20S%20Replies%20Structures))
  (Utilities|Struct|SetmembersinS_DialogueContent (Utilities|Array|Get(acopy) (Variables|Default|GetDialogue%20Content) Index) "NewEnumerator2" Replies)
  (return))

(fn ClearDialogue
  (Utilities|Array|Clear (Variables|Default|GetDialogue%20Content)))

(fn IncrementTimesSpokenwithLimit
  (params (Limit :type Integer))
  (bind _times_spoken (Variables|Default|GetTimes%20Spoken))
  (if (< _times_spoken Limit)
    (Math|Integer|IncrementInt _times_spoken)))

(fn GetRandomIntWithoutRepeating
  (params (Max :type Integer))
  (bind _n (Variables|Default|GetN))
  (if (< (Utilities|Array|Length (Variables|Default|GetInt%20Array)) 1)
    (while (< (Variables|Default|GetN) Max)
      (Utilities|Array|Add (Variables|Default|GetInt%20Array) _n)
      (Math|Integer|IncrementInt _n))
    (Utilities|FlowControl|Sequence
      (:then_0
        (Utilities|FlowControl|DoOnce false
          (:Completed
            (Variables|Default|SetRandom%20Array (Variables|Default|GetInt%20Array)))))
      (:then_1
        (bind _output_get (LocalVariables|SetTemp%20Int (.OutItem (Utilities|Array|Random (Variables|Default|GetRandom%20Array))) :!label _label))
        (bind _output_get_2 (Variables|Default|SetRandom%20Array (Variables|Default|GetInt%20Array)))
        (Utilities|Array|RemoveItem _output_get_2 _output_get)
        (return (LocalVariables|GetTemp%20Int))))
    (else
      (goto _label))))