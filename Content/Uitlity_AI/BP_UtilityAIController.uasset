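; Utility AI controller that picks and runs the highest-scoring task for its controlled pawn.
; On BeginPlay it instantiates each class in Tasks into TaskList, if that list is empty, then evaluates a decision.
; CalculateDecision scores every task against the UAIBB object; when the winner differs from CurrentTask, it aborts the current one and executes the winner.
; This graph triggers evaluation only at BeginPlay, with no tick or timer.
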(event Custom|Calculate%20Decision
  (bind _new_task (CallFunction|CalculateTaskScore))
  (if (!= _new_task (Variables|Default|GetCurrent%20Task))
    (bind _current_task (Variables|Default|GetCurrent%20Task)
      (:then
        (Default|AbortAI _current_task))
      (:else
        _))
    (Variables|Default|SetCurrent%20Task _new_task)
    (CallFunction|RunTask)))

(event EventBeginPlay
  ;[1 1 1] Begin Play
  (if (> (Utilities|Array|Length (Variables|Default|GetTask%20List)) 0)
    _
    (else
      (for _array_element (Variables|Default|GetTasks)
        (bind _returnvalue (Game|ConstructObjectfromClass _array_element self))
        (Utilities|Array|AddUnique (Variables|Default|GetTask%20List) _returnvalue))))
  (CallFunction|CalculateDecision))

(fn ConstructionScript)

(fn CalculateTaskScore
  (for _array_element (Variables|Default|GetTask%20List)
    (bind _task_score (Default|CalculateTask _array_element (Variables|Default|GetUAIBB)))
    (if (> _task_score (LocalVariables|GetHighest%20Task%20Score))
      (LocalVariables|SetHighest%20Task%20Score _task_score)
      (LocalVariables|SetTemp%20New%20Task _array_element)))
  (return (LocalVariables|GetTemp%20New%20Task)))

(fn RunTask
  (Default|ExecuteAI (Variables|Default|GetCurrent%20Task) self (Pawn|GetControlledPawn) (Variables|Default|GetUAIBB)))